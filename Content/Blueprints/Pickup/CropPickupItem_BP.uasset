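; CropPickupItem_BP is a crop pickup actor; its graph only drives a development-only label showing the item's crop type.
; On BeginPlay, RenderPlantItemText writes the CropType enum name into the ItemRenderText_UI widget held by TextWidget.
; Tick, throttled by a one-second Delay, rewrites the label while it still reads "None", intended for items spawned after combat.
; Both label paths are marked for removal before production.
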(event Custom|RenderPlantItemText
  ;[1 0 0.1827] DEVELOPMENT ONLY: This just shows the Crop Type - Remove for Prod
  (bind _asitem_render_text_ui (Utilities|Casting|CastToItemRenderText_UI (UserInterface|GetUserWidgetObject (Variables|Default|GetTextWidget))))
  (Rendering|Components|TextRender|SetText (Variables|/Game/Blueprints/Pickup/ItemRenderText_UI.ItemRenderText_UI_C|GetRenderText _asitem_render_text_ui) (Utilities|Text|ToText(String) (Utilities|String|EnumtoString (Variables|Default|GetCropType)))))

(event EventBeginPlay
  (CallFunction|RenderPlantItemText))

(event Collision|EventActorBeginOverlap
  (params (OtherActor :type Actor%20Object%20Reference)))

(event EventTick
  (params (DeltaSeconds :type Float%20%28single-precision%29))
  ;[1 0 0.1538] Development only: This shows the croptype on the spawned item after combat - Remove for Prod
  (Utilities|FlowControl|Delay 1.0)
  (bind _asitem_render_text_ui (Utilities|Casting|CastToItemRenderText_UI (UserInterface|GetUserWidgetObject (Variables|Default|GetTextWidget))))
  (if (Utilities|Enum|Equal(Enum) (Class|TextBlock|GetText (Variables|/Game/Blueprints/Pickup/ItemRenderText_UI.ItemRenderText_UI_C|GetRenderText _asitem_render_text_ui)) (Utilities|Text|MakeLiteralText "None"))
    (CallFunction|RenderPlantItemText)))

(fn ConstructionScript)