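; MainPlayerController_BP is a player controller with test key bindings for cursor modes and a planting-mode camera check.
; F sets a TargetReticle_UI widget as the crosshair cursor, and G switches to the default hardware cursor.
; H moves MainCharacter_BP's camera boom to a longer, fixed-pitch view, and I returns it to control-rotation follow.
; J prints the impact point of a visibility trace under the cursor.
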(event EventBeginPlay)

(event EventTick
  (params (DeltaSeconds :type Float%20%28single-precision%29)))

(event Input|ActionEvents|InputActionFKey
  (params (Key :type Key%20Structure :default "None"))
  (:Pressed
    (Utilities|Casting|CastToMainCharacter_BP (Game|GetPlayerCharacter 0))
    (bind _returnvalue (UserInterface|CreateWidget "/Game/Blueprints/UI/TargetReticle_UI.TargetReticle_UI_C"))
    (bind _output_get (Variables|Default|SetReticleWidgetRef _returnvalue))
    (bind _output_get_2 (Variables|Default|SetCurrentMouseCursor "Crosshairs"))
    (Class|PlayerController|SetMouseCursorWidget _output_get_2 _output_get)
    (Variables|Default|SetbShowMouseCursor true)
    (Development|PrintString "Hello")))

(event Input|KeyboardEvents|G
  (params (Key :type Key%20Structure :default "None"))
  (:Pressed
    (Utilities|Casting|CastToMainCharacter_BP (Game|GetPlayerCharacter 0))
    (bind _output_get (Variables|Default|SetCurrentMouseCursor "Default"))
    (Class|WidgetBlueprintLibrary|SetHardwareCursor _output_get "Default")
    (Variables|Default|SetbShowMouseCursor true)
    (Development|PrintString "Goodbye")))

(event Input|KeyboardEvents|H
  (params (Key :type Key%20Structure :default "None"))
  ;[1 0 0.06651] DEBUG: Camera shift check for planting mode
  (:Pressed
    (bind _asmain_character_bp (Utilities|Casting|CastToMainCharacter_BP (Game|GetPlayerCharacter 0)))
    (Variables|/Script/Engine.SpringArmComponent|SetbUsePawnControlRotation (Variables|/Script/CursedHarvest.MainCharacter|GetCameraBoom _asmain_character_bp) false)
    (Variables|/Script/Engine.SpringArmComponent|SetTargetArmLength (Variables|/Script/CursedHarvest.MainCharacter|GetCameraBoom _asmain_character_bp) 4e+02)
    (Transformation|SetRelativeRotation (Variables|/Script/CursedHarvest.MainCharacter|GetCameraBoom _asmain_character_bp) "-60.000000, 0, 0" false false)))

(event Input|KeyboardEvents|I
  (params (Key :type Key%20Structure :default "None"))
  ;[1 0 0.06651] DEBUG: Camera shift check for planting mode
  (:Pressed
    (bind _asmain_character_bp (Utilities|Casting|CastToMainCharacter_BP (Game|GetPlayerCharacter 0)))
    (Variables|/Script/Engine.SpringArmComponent|SetbUsePawnControlRotation (Variables|/Script/CursedHarvest.MainCharacter|GetCameraBoom _asmain_character_bp) true)
    (Variables|/Script/Engine.SpringArmComponent|SetTargetArmLength (Variables|/Script/CursedHarvest.MainCharacter|GetCameraBoom _asmain_character_bp) 3e+02)
    (Transformation|SetRelativeRotation (Variables|/Script/CursedHarvest.MainCharacter|GetCameraBoom _asmain_character_bp) "0, 0, 0" false false)))

(event Input|KeyboardEvents|J
  (params (Key :type Key%20Structure :default "None"))
  (:Pressed
    (Development|PrintString (Utilities|String|ToString(Vector) (.ImpactPoint (Collision|BreakHitResult (.HitResult (Game|Player|GetHitResultUnderCursorbyChannel "TraceTypeQuery1" true))))))))

(fn ConstructionScript)